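; Player component for an instant photo camera with viewfinder, zoom, flash toggle, traced autofocus and a pausing photo gallery.
; Montage notifies drive aiming, printing and grabbing, while timelines animate the print, development and head turns.
; Shooting captures the scene to a render target, exports it to Saved/Pictures and shows it on the photo's dynamic material.
; A BP_PhotoGallery save game tracks picture numbers for the photo limit and deletion.
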(event Custom|ShootAndReceivePicture
  ;[0 0.7682 1] Print and develop photo / control animation montage
  (Variables|MainVariables|SetPictureMode false)
  (Utility|CameraFlash)
  (Utilities|FlowControl|Sequence
    (:then_0
      (CallFunction|DisablePictureMode false))
    (:then_1
      ;;[1 1 1] Wait for fade animation and attach camera to print socket (in player hand)
      (Utilities|FlowControl|Delay 0.2)
      (Transformation|AttachComponentToComponent (Variables|Default|GetCameraMesh) (Variables|Default|GetPlayerMesh) "CameraSocket_Print" "SnapToTarget" "SnapToTarget" "KeepRelative" true)
      ;;[1 1 1] Disable Input, take picture and attach it to Camera
      (Input|DisableInput (Game|Player|GetPlayerPawn 0) (Game|GetPlayerController 0))
      (TakingPicture|TakePicture)
      (TakingPicture|AttachPhototoCamera)
      ;;[1 1 1] Control photo animation montage - print, develop, take
      (bind _notifyname (Animation|Montage|PlayMontage (Variables|Default|GetPlayerMesh) (Variables|Setup|GetAnimMontage) 1.0 0.0 "PrintPicture")
        (:OnNotifyBegin
          (switch name _notifyname
            (:PrintPhoto
              (|PrintPhotoAnimation
                (:Finished
                  (|DevelopPhoto(Material)))))
            (:GrabbedPhoto
              (Transformation|AttachComponentToComponent (Variables|Default|GetPhotoMesh) (Variables|Default|GetPlayerMesh) "PictureSocket" "KeepWorld" "KeepWorld" "KeepRelative" true) ; Attach photo to player hand (PictureSocket)
            )
            (:LookAtPhoto
              (CallFunction|LookatPhoto))))))
    (:then_2
      ;;[1 1 1] Turn head to camera in hand after fade animation
      (Utilities|FlowControl|Delay 0.4)
      (CallFunction|LookatCamera)
      ;;[1 1 1] Un crouch
      (bind _ascharacter (Utilities|Casting|CastToCharacter (Actor|GetParentActor)))
      (Character|UnCrouch _ascharacter))))

(event Custom|SetCamera
  (bind _cameramesh (Variables|Default|GetCameraMesh))
  ;[0 0.7682 1] Set Camera: Bind Camera to Player Character and Play Aim Montage
  (Transformation|AttachComponentToComponent _cameramesh (Variables|Default|GetPlayerMesh) "CameraSocket_Hold" "SnapToTarget" "SnapToTarget" "KeepRelative" true)
  (Rendering|SetVisibility _cameramesh true false)
  (Rendering|SetCastShadow _cameramesh true)
  (bind _notifyname (Animation|Montage|PlayMontage (Variables|Default|GetPlayerMesh) (Variables|Setup|GetAnimMontage) 1.0 0.0 "SetCamera")
    (:OnNotifyBegin
      (if (Utilities|Name|Equal(Name) _notifyname "PhotoMode")
        (CallFunction|EnablePictureMode)))))

(event Custom|UnsetCamera
  ;[0 0.7682 1] Unset camera
  (CallFunction|DisablePictureMode true)
  (Utilities|FlowControl|Delay 0.4)
  (Animation|Montage|PlayMontage (Variables|Default|GetPlayerMesh) (Variables|Setup|GetAnimMontage) -0.5 0.0 "1.3"))

(event Custom|EnablePictureMode
  ;[0 0.7682 1] Enable Picture Mode
  (bind _returnvalue (UserInterface|CreateWidget "/Game/InstantPhotoCamera/UserInterface/WBP_Viewfinder.WBP_Viewfinder_C"))
  (bind _output_get (Variables|References|SetViewfinderHUD _returnvalue))
  (UserInterface|Viewport|AddtoViewport _output_get 0)
  (Utilities|FlowControl|Delay 0.25)
  (Rendering|SetVisibility (Variables|Default|GetCameraMesh) false false)
  (Default|ToggleFlashIcon (Variables|References|GetViewfinderHUD) (Variables|MainVariables|GetFlashEnabled))
  (Effects|AdjustCameraforPictureMode)
  (Utilities|FlowControl|Delay 0.2)
  (Variables|MainVariables|SetPictureMode true)
  (bind _returnvalue_2 (Utilities|Time|SetTimerbyEvent (EventDispatchers|CreateEvent :!event SetFocalDistance) 0.01 true)) ; Constantly adjust focal distance while in picture mode
  (Variables|MainVariables|SetFocalDistanceTimer _returnvalue_2))

(event Custom|DisablePictureMode
  (params (HideCamera :type Boolean))
  (bind _cameramesh (Variables|Default|GetCameraMesh))
  ;[0 0.7379 1] Disable Picture Mode
  (Variables|MainVariables|SetPictureMode false)
  (Utilities|Time|ClearandInvalidateTimerbyHandle (Variables|MainVariables|GetFocalDistanceTimer)) ; Stop adjusting focal distance
  (bind _viewfinderhud (Variables|References|GetViewfinderHUD)
    (:then
      (UserInterface|Animation|PlayAnimation _viewfinderhud (Variables|/Game/InstantPhotoCamera/UserInterface/WBP_Viewfinder.WBP_Viewfinder_C|GetFade _viewfinderhud) 0.8 1 "Reverse" 1.0 false)
      (Utilities|FlowControl|Delay 0.4))
    (:else
      _))
  (Effects|ResetCameraEffects)
  (Utilities|FlowControl|Delay 0.4)
  (Widget|RemovefromParent (Variables|References|GetViewfinderHUD))
  (if HideCamera
    (Rendering|SetVisibility _cameramesh false false)
    (Rendering|SetCastShadow _cameramesh false)))

(event Custom|CameraFull
  ;[0 0.7682 1] Camera full
  (Utilities|FlowControl|DoOnce false :!label _label
    (:Completed
      (bind _returnvalue (UserInterface|CreateWidget "/Game/InstantPhotoCamera/UserInterface/WBP_CameraScreenMessages.WBP_CameraScreenMessages_C"))
      (UserInterface|Viewport|AddtoViewport _returnvalue 0)
      (UserInterface|Animation|PlayAnimation _returnvalue (Variables|/Game/InstantPhotoCamera/UserInterface/WBP_CameraScreenMessages.WBP_CameraScreenMessages_C|GetFade _returnvalue) 0.0 1 "Forward" 1.0 false)
      (Utilities|FlowControl|Delay (Class|WidgetAnimation|GetEndTime (Variables|/Game/InstantPhotoCamera/UserInterface/WBP_CameraScreenMessages.WBP_CameraScreenMessages_C|GetFade _returnvalue)))
      (Widget|RemovefromParent _returnvalue)
      (goto _label Reset))))

(event Custom|LookAtCamera
  ;[0 0.7682 1] Look at Camera
  (Variables|MainVariables|SetCameraOriginRotation (Pawn|GetControlRotation (Game|GetPlayerController 0) :!class /Script/Engine.Controller))
  (bind _alphacurve (Timeline|LookAtCameraTimeline PlayFromStart)
    (:Update
      (Pawn|SetControlRotation (Game|GetPlayerController 0) (Math|Rotator|Lerp(Rotator) (Variables|MainVariables|GetCameraOriginRotation) (Math|Rotator|MakeRotator (.Roll (Math|Rotator|BreakRotator (Variables|MainVariables|GetCameraOriginRotation))) -6e+01 (.Yaw (Math|Rotator|BreakRotator (Variables|MainVariables|GetCameraOriginRotation)))) _alphacurve true)))))

(event Custom|LookAtPhoto
  (bind _returnvalue (Game|GetPlayerController 0))
  ;[0 0.7682 1] Look at Photo
  (Variables|MainVariables|SetLookAtCameraRotation (Pawn|GetControlRotation (Game|GetPlayerController 0) :!class /Script/Engine.Controller))
  (bind _alphacurve (Timeline|LookAtPhotoTimeline PlayFromStart)
    (:Update
      (Pawn|SetControlRotation (Game|GetPlayerController 0) (Math|Rotator|Lerp(Rotator) (Variables|MainVariables|GetLookAtCameraRotation) (Math|Rotator|MakeRotator (.Roll (Math|Rotator|BreakRotator (Variables|MainVariables|GetLookAtCameraRotation))) (+ (.Pitch (Math|Rotator|BreakRotator (Variables|MainVariables|GetLookAtCameraRotation))) 4e+01) (.Yaw (Math|Rotator|BreakRotator (Variables|MainVariables|GetLookAtCameraRotation)))) _alphacurve)))
    (:Finished
      ;[0 0.7682 1] Enable input and hide camera and photo
      (Utilities|FlowControl|Delay 2.0)
      (Rendering|SetVisibility (Variables|Default|GetPhotoMesh) false false)
      (Rendering|SetCastShadow (Variables|Default|GetCameraMesh) false)
      (Input|EnableInput (Game|Player|GetPlayerPawn 0) _returnvalue)
      (Input|EnableInput _returnvalue))))

(event EventBeginPlay
  (bind _returnvalue (Actor|GetParentActor))
  ;[0 0.7682 1] Create Dynamic Material Instance and attach Capture Component to Player Character
  (bind _returnvalue_2 (Rendering|Material|CreateDynamicMaterialInstance (Variables|Default|GetPhotoMesh) 0 "/Game/InstantPhotoCamera/Materials/M_InstantPhoto.M_InstantPhoto" "None" :!class /Script/Engine.PrimitiveComponent))
  (Variables|References|SetMaterial _returnvalue_2)
  (Variables|Default|SetPlayerMesh (Actor|GetComponentbyClass _returnvalue "/Script/Engine.SkeletalMeshComponent"))
  (bind _output_get (Variables|Default|SetPlayerCamera (Actor|GetComponentbyClass _returnvalue "/Script/Engine.CameraComponent")))
  (bind _output_get_2 (Variables|MainVariables|SetGameFoV (Variables|/Script/Engine.CameraComponent|GetFieldOfView _output_get)))
  (Variables|MainVariables|SetCaptureFieldOfView _output_get_2)
  (bind _output_get_3 (Variables|PostProcess|SetGamePostProcess (Variables|/Script/Engine.CameraComponent|GetPostProcessSettings (Variables|Default|GetPlayerCamera))))
  (Variables|/Script/Engine.SceneCaptureComponent2D|SetPostProcessSettings (Variables|Default|GetCaptureComponent) _output_get_3)
  (Variables|MainVariables|SetCameraOriginLocation (Variables|/Script/Engine.SceneComponent|GetRelativeLocation (Variables|Default|GetPlayerCamera)))
  (Transformation|AttachComponentToComponent (Variables|Default|GetCaptureComponent) (Variables|Default|GetPlayerCamera) "" "SnapToTarget" "SnapToTarget" "KeepRelative" true))

(event Input|ActionEvents|InputActionZoomIn
  (params (Key :type Key%20Structure))
  ;[0 0.7682 1] Zoom in and out
  (:Pressed
    (if (Variables|MainVariables|GetPictureMode)
      (FieldofView|ChangeFieldOfView -2e+01))))

(event Input|ActionEvents|InputActionSetCamera
  (params (Key :type Key%20Structure))
  ;[0 0.7682 1] Input: Set Camera
  (:Pressed
    (Utilities|Cooldown 2.0
      (:Completed
        (if (Utility|ReachedMaxPictures)
          (CallFunction|CameraFull)
          (elif (Variables|MainVariables|GetPictureMode)
            (CallFunction|UnsetCamera)
            (else
              (CallFunction|SetCamera))))))))

(event Input|ActionEvents|InputActionToggleCameraFlash
  (params (Key :type Key%20Structure))
  ;[0 0.7682 1] Input: Toggle Camera Flash
  (:Pressed
    (if (Variables|MainVariables|GetPictureMode)
      (if (Variables|MainVariables|GetFlashEnabled)
        (Variables|MainVariables|SetFlashEnabled false)
        (else
          (Variables|MainVariables|SetFlashEnabled true)))
      (Default|ToggleFlashIcon (Variables|References|GetViewfinderHUD) (Variables|MainVariables|GetFlashEnabled)))))

(event Input|ActionEvents|InputActionShootPhoto
  (params (Key :type Key%20Structure))
  ;[0 0.7682 1] Input: Take Picture
  (:Pressed
    (if (Variables|MainVariables|GetPictureMode)
      (Input|DisableInput (Game|GetPlayerController 0))
      (CallFunction|ShootandReceivePicture))))

(event Input|ActionEvents|InputActionGalleryPrevPage
  (params (Key :type Key%20Structure))
  ;[0 0.7682 1] Photo Gallery Control
  (:Pressed
    (bind _galleryhud (Variables|References|GetGalleryHUD)
      (:then
        (bind _playsound (Default|SetPrevPage _galleryhud))
        (if _playsound
          (Audio|PlaySound2D "/Game/InstantPhotoCamera/Sounds/Cues/SC_TurnPage.SC_TurnPage" 1.0 1.0 0.0 0 0)))
      (:else))))

(event Input|ActionEvents|InputActionZoomOut
  (params (Key :type Key%20Structure))
  ;[0 0.7682 1] Zoom in and out
  (:Pressed
    (if (Variables|MainVariables|GetPictureMode)
      (FieldofView|ChangeFieldOfView 2e+01))))

(event Input|ActionEvents|InputActionGallery
  (params (Key :type Key%20Structure))
  ;[0 0.7682 1] Photo Gallery Control
  (:Pressed
    (if (not (Variables|MainVariables|GetPictureMode))
      (PhotoGallery|ToggleGallery Key))))

(event Input|ActionEvents|InputActionGalleryNextPage
  (params (Key :type Key%20Structure))
  ;[0 0.7682 1] Photo Gallery Control
  (:Pressed
    (bind _galleryhud (Variables|References|GetGalleryHUD)
      (:then
        (bind _playsound (Default|SetNextPage _galleryhud))
        (if _playsound
          (Audio|PlaySound2D "/Game/InstantPhotoCamera/Sounds/Cues/SC_TurnPage.SC_TurnPage" 1.0 1.0 0.0 0 0)))
      (:else))))

(fn ConstructionScript
  (Components|Timeline|SetPlayRate (Variables|Default|GetDevelopPhotoTimeline) (.developtime (Variables|Setup|GetCameraSettings)))
  (Variables|/Script/Engine.TextureRenderTarget|SetTargetGamma (Variables|/Script/Engine.SceneCaptureComponent2D|GetTextureTarget (Variables|Default|GetCaptureComponent)) (.brightnesscorrection (Variables|Setup|GetCameraSettings))))

(fn DeleteSelectedPicture
  (params (PictureNumber :type Integer))
  (LocalVariables|SetPicture PictureNumber)
  (bind _returnvalue (SaveGame|LoadGamefromSlot (Variables|MainVariables|GetSaveGameSlot)))
  (bind _asbp_photo_gallery (Utilities|Casting|CastToBP_PhotoGallery _returnvalue))
  (Variables|References|SetGallerySaveGame _asbp_photo_gallery)
  (Class|BlueprintFileUtilsBPLibrary|DeleteFile (Utilities|String|Append (Utilities|String|Append (Class|KismetSystemLibrary|GetProjectSavedDirectory) "/Pictures") "/pic_" (Utilities|String|ToString(Integer) (LocalVariables|GetPicture))) true false)
  (Variables|/Game/InstantPhotoCamera/Blueprints/BP_PhotoGallery.BP_PhotoGallery_C|SetPictureCount (Variables|References|GetGallerySaveGame) (- (Variables|/Game/InstantPhotoCamera/Blueprints/BP_PhotoGallery.BP_PhotoGallery_C|GetPictureCount (Variables|References|GetGallerySaveGame)) 1))
  (Utilities|Array|RemoveItem (Variables|/Game/InstantPhotoCamera/Blueprints/BP_PhotoGallery.BP_PhotoGallery_C|GetPictureNumbers (Variables|References|GetGallerySaveGame)) (LocalVariables|GetPicture))
  (SaveGame|SaveGametoSlot (Variables|References|GetGallerySaveGame) (Variables|MainVariables|GetSaveGameSlot)))

(fn ToggleGallery
  (params (Key :type Key%20Structure :default "None"))
  (bind _returnvalue (Game|GetPlayerController 0))
  (bind _returnvalue_2 (Game|GetPlayerController 0))
  (LocalVariables|SetKeyboardInput (Class|KismetInputLibrary|KeyIsKeyboardKey Key))
  (Utilities|IsValid (Variables|References|GetGalleryHUD)
    (:Is%20Valid
      (Widget|RemovefromParent (Variables|References|GetGalleryHUD))
      (Variables|References|SetGalleryHUD 0)
      (Audio|PlaySound2D "/Game/InstantPhotoCamera/Sounds/Cues/SC_CloseBook.SC_CloseBook" 1.0 1.0 0.0 0 0)
      (Game|SetGamePaused false)
      (Variables|/Script/Engine.PlayerController|SetbShowMouseCursor _returnvalue_2 false)
      (Input|SetInputModeGameOnly _returnvalue_2)
      (bind _foundwidgets (Widget|GetAllWidgetsOfClass "/Game/InstantPhotoCamera/UserInterface/WBP_InstantPhotoFullscreen.WBP_InstantPhotoFullscreen_C" true))
      (if (Utilities|Array|IsValidIndex _foundwidgets)
        (Widget|RemovefromParent (Utilities|Array|Get(acopy) _foundwidgets))))
    (:Is%20Not%20Valid
      (if (not (Game|IsGamePaused))
        (bind _returnvalue_3 (UserInterface|CreateWidget "/Game/InstantPhotoCamera/UserInterface/WBP_PhotoGallery.WBP_PhotoGallery_C" 0 (LocalVariables|GetKeyboardInput)))
        (bind _output_get (Variables|References|SetGalleryHUD _returnvalue_3))
        (UserInterface|Viewport|AddtoViewport _output_get 0)
        (Audio|PlaySound2D "/Game/InstantPhotoCamera/Sounds/Cues/SC_OpenBook.SC_OpenBook" 1.0 1.0 0.0 0 0)
        (Game|SetGamePaused true)
        (if (LocalVariables|GetKeyboardInput)
          (Variables|/Script/Engine.PlayerController|SetbShowMouseCursor _returnvalue true)
          (Input|SetInputModeGameandUI _returnvalue (Variables|References|GetGalleryHUD) "DoNotLock" true))))))

(fn FieldOfViewInterpolation
  (bind _returnvalue (Utilities|Time|GetWorldDeltaSeconds))
  (bind _playercamera (Variables|Default|GetPlayerCamera))
  (bind _targetfieldofview (Variables|MainVariables|GetTargetFieldOfView))
  (bind _fieldofview (Variables|/Script/Engine.CameraComponent|GetFieldOfView _playercamera))
  (bind _returnvalue_2 (Math|Interpolation|FInterpTo _fieldofview _targetfieldofview _returnvalue 5.0))
  (if (Math|Float|NearlyEqual(Float) _fieldofview _targetfieldofview 0.01)
    (Utilities|Time|ClearTimerbyFunctionName 0 "FieldOfViewInterpolation")
    (else
      (Camera|SetFieldOfView (Variables|Default|GetPlayerCamera) _returnvalue_2)
      (Default|ChangeZoomFactor (Variables|References|GetViewfinderHUD) (- 5 (Math|Float|Round (* (Math|Float|NormalizetoRange _returnvalue_2 2e+01 8e+01) 3.333333)))))))

(fn SetFocalDistance
  (bind _returnvalue (Game|GetPlayerCameraManager 0))
  (bind _returnvalue_2 (Transformation|GetActorLocation _returnvalue))
  (if (Variables|MainVariables|GetPictureMode)
    (bind (_outhit _returnvalue_3) (Collision|LineTraceByChannel _returnvalue_2 (+ _returnvalue_2 (* (Transformation|GetActorForwardVector _returnvalue) 5e+03)) "TraceTypeQuery1" false 0 "None"))
    (bind _output_get (Variables|PostProcess|SetTargetFocalDistance (select _returnvalue_3 (.Distance (Collision|BreakHitResult _outhit)) 5e+03)))
    (bind _output_get_2 (Variables|PostProcess|SetCurrentFocalDistance (Math|Interpolation|FInterpTo (Variables|PostProcess|GetCurrentFocalDistance) _output_get (Utilities|Time|GetWorldDeltaSeconds) 6.0)))
    (Utilities|Struct|SetmembersinPostProcessSettings (Variables|/Script/Engine.CameraComponent|GetPostProcessSettings (Variables|Default|GetPlayerCamera)) 1.2 _output_get_2 5e+01)
    (Utilities|Struct|SetmembersinPostProcessSettings (Variables|/Script/Engine.SceneCaptureComponent2D|GetPostProcessSettings (Variables|Default|GetCaptureComponent)) (Variables|PostProcess|GetCurrentFocalDistance))))

(fn ResetCameraEffects
  (Utilities|Time|ClearTimerbyFunctionName 0 "FieldOfViewInterpolation")
  (Camera|SetFieldOfView (Variables|Default|GetPlayerCamera) (Variables|MainVariables|GetGameFoV))
  (Variables|/Script/Engine.CameraComponent|SetPostProcessSettings (Variables|Default|GetPlayerCamera) (Variables|PostProcess|GetGamePostProcess))
  (Transformation|SetRelativeLocation (Variables|Default|GetPlayerCamera) (Variables|MainVariables|GetCameraOriginLocation) false false))

(fn AdjustCameraforPictureMode
  ;[1 1 1] Adjust picture field of view to camera field of view
  (Variables|/Script/Engine.SceneCaptureComponent2D|SetFOVAngle (Variables|Default|GetCaptureComponent) (* (Variables|/Script/Engine.CameraComponent|GetFieldOfView (Variables|Default|GetPlayerCamera)) (Variables|MainVariables|GetFieldOfViewConversionFactor)))
  ;[1 1 1] Prevent camera from clipping through players hands
  (Transformation|SetRelativeLocation (Variables|Default|GetPlayerCamera) (+ (Variables|MainVariables|GetCameraOriginLocation) "0,25.000000, 0") false false))

(fn ChangeFieldOfView
  (params (Value :type Float%20%28single-precision%29))
  (bind _output_get (LocalVariables|SetFoVChange Value))
  (bind _output_get_2 (Variables|MainVariables|SetTargetFieldOfView (Math|Float|ClampAngle (+ (Variables|/Script/Engine.CameraComponent|GetFieldOfView (Variables|Default|GetPlayerCamera)) _output_get) 2e+01 (Variables|MainVariables|GetGameFoV))))
  (Variables|/Script/Engine.SceneCaptureComponent2D|SetFOVAngle (Variables|Default|GetCaptureComponent) (* _output_get_2 (Variables|MainVariables|GetFieldOfViewConversionFactor)))
  (Utilities|Time|SetTimerbyFunctionName 0 "FieldOfViewInterpolation" 0.01 true))

(fn DeleteAllPictures
  ;[0 0.7379 1] Remove all pictures in folder and delete save game
  (bind _returnvalue (SaveGame|DoesSaveGameExist (Variables|MainVariables|GetSaveGameSlot)))
  (if _returnvalue
    (bind _returnvalue_2 (SaveGame|LoadGamefromSlot (Variables|MainVariables|GetSaveGameSlot)))
    (bind _asbp_photo_gallery (Utilities|Casting|CastToBP_PhotoGallery _returnvalue_2))
    (Variables|References|SetGallerySaveGame _asbp_photo_gallery)
    (for _array_element (Variables|/Game/InstantPhotoCamera/Blueprints/BP_PhotoGallery.BP_PhotoGallery_C|GetPictureNumbers (Variables|References|GetGallerySaveGame))
      (Class|BlueprintFileUtilsBPLibrary|DeleteFile (Utilities|String|Append (Utilities|String|Append (Class|KismetSystemLibrary|GetProjectSavedDirectory) "/Pictures") "/pic_" (Utilities|String|ToString(Integer) _array_element)) true false))
    (SaveGame|DeleteGameinSlot (Variables|MainVariables|GetSaveGameSlot))))

(fn AddPictureCount
  (bind _returnvalue (SaveGame|DoesSaveGameExist (Variables|MainVariables|GetSaveGameSlot)))
  (if _returnvalue
    (bind _returnvalue_2 (SaveGame|LoadGamefromSlot (Variables|MainVariables|GetSaveGameSlot)))
    (bind _asbp_photo_gallery (Utilities|Casting|CastToBP_PhotoGallery _returnvalue_2))
    (Variables|References|SetGallerySaveGame _asbp_photo_gallery)
    (else
      (bind _returnvalue_3 (SaveGame|CreateSaveGameObject "/Game/InstantPhotoCamera/Blueprints/BP_PhotoGallery.BP_PhotoGallery_C"))
      (Variables|References|SetGallerySaveGame _returnvalue_3)))
  (Variables|/Game/InstantPhotoCamera/Blueprints/BP_PhotoGallery.BP_PhotoGallery_C|SetPictureCount (Variables|References|GetGallerySaveGame) (+ (Variables|/Game/InstantPhotoCamera/Blueprints/BP_PhotoGallery.BP_PhotoGallery_C|GetPictureCount (Variables|References|GetGallerySaveGame)) 1))
  (Utilities|FlowControl|Sequence
    (:then_0
      (LocalVariables|SetNextNumber (+ (Utilities|Array|Get(acopy) (Variables|/Game/InstantPhotoCamera/Blueprints/BP_PhotoGallery.BP_PhotoGallery_C|GetPictureNumbers (Variables|References|GetGallerySaveGame)) (Utilities|Array|LastIndex (Variables|/Game/InstantPhotoCamera/Blueprints/BP_PhotoGallery.BP_PhotoGallery_C|GetPictureNumbers (Variables|References|GetGallerySaveGame)))) 1)))
    (:then_1
      (Utilities|Array|AddUnique (Variables|/Game/InstantPhotoCamera/Blueprints/BP_PhotoGallery.BP_PhotoGallery_C|GetPictureNumbers (Variables|References|GetGallerySaveGame)) (LocalVariables|GetNextNumber))
      (SaveGame|SaveGametoSlot (Variables|References|GetGallerySaveGame) (Variables|MainVariables|GetSaveGameSlot))
      (return (LocalVariables|GetNextNumber)))))

(fn CameraFlash
  ;[0 0.7379 1] If flash is enabled, show camera flash light
  (if (Variables|MainVariables|GetFlashEnabled)
    (Rendering|SetVisibility (Variables|Default|GetCameraFlashComponent) true false)))

(fn StopCameraFlash
  (Rendering|SetVisibility (Variables|Default|GetCameraFlashComponent) false false))

(fn ReachedMaxPictures
  (bind _returnvalue (SaveGame|DoesSaveGameExist (Variables|MainVariables|GetSaveGameSlot)))
  (if _returnvalue
    (bind _returnvalue_2 (SaveGame|LoadGamefromSlot (Variables|MainVariables|GetSaveGameSlot)))
    (bind _asbp_photo_gallery (Utilities|Casting|CastToBP_PhotoGallery _returnvalue_2))
    (if (== (Variables|/Game/InstantPhotoCamera/Blueprints/BP_PhotoGallery.BP_PhotoGallery_C|GetPictureCount _asbp_photo_gallery) (.maxpictures (Variables|Setup|GetCameraSettings)))
      (return true)
      (else
        _)))
  (return false))

(fn TakePicture
  (bind _capturecomponent (Variables|Default|GetCaptureComponent))
  ;[0 0.7682 1] Set Photo Number, create a new Render Target Asset -> set as Texture Target, set Scene Capture as Photo Image and save to Gallery
  (Rendering|SceneCapture|CaptureScene _capturecomponent :!class /Script/Engine.SceneCaptureComponent2D)
  (bind _number (TakingPicture|AddPictureCount))
  (Rendering|ExportRenderTarget (Variables|/Script/Engine.SceneCaptureComponent2D|GetTextureTarget _capturecomponent) (Utilities|String|Append (Class|KismetSystemLibrary|GetProjectSavedDirectory) "/Pictures") (Utilities|String|Append "pic_" (Utilities|String|ToString(Integer) _number)))
  (Rendering|Material|SetTextureParameterValue (Variables|References|GetMaterial) "Picture" (Variables|/Script/Engine.SceneCaptureComponent2D|GetTextureTarget (Variables|Default|GetCaptureComponent)))
  (Audio|PlaySoundatLocation "/Game/InstantPhotoCamera/Sounds/Cues/SC_ShootPhoto.SC_ShootPhoto" (Transformation|GetWorldLocation (Variables|Default|GetCameraMesh)) "0, 0, 0" 1.0 1.0 0.0 0 0 0)
  (Utility|StopCameraFlash))

(fn AttachPhototoCamera
  (Rendering|SetVisibility (Variables|Default|GetCameraMesh) true false)
  (Transformation|AttachComponentToComponent (Variables|Default|GetPhotoMesh) (Variables|Default|GetCameraMesh) "None" "SnapToTarget" "SnapToTarget" "KeepRelative" true)
  (Transformation|SetRelativeLocation (Variables|Default|GetPhotoMesh) "0, 0,2.000000" false false)
  (Rendering|Material|SetScalarParameterValue (Variables|References|GetMaterial) "Transition" 0.0 :!class /Script/Engine.MaterialInstanceDynamic)
  (Rendering|SetVisibility (Variables|Default|GetPhotoMesh) true false))