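; BP_InstantPhoto displays a picture from the instant camera's saved photo gallery on its photo mesh.
; On BeginPlay it loads the "CMRA" gallery save and picks either a random entry or the configured photo number.
; It imports the matching image from the project's Saved Pictures folder at runtime and feeds it to a dynamic material, setting the transition to fully on.
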(event Custom|SetPicture
  ;[1 1 1] Load Gallery Save Game
  (bind _returnvalue (SaveGame|DoesSaveGameExist "CMRA"))
  (if _returnvalue
    (bind _returnvalue_2 (SaveGame|LoadGamefromSlot "CMRA"))
    (bind _asbp_photo_gallery (Utilities|Casting|CastToBP_PhotoGallery _returnvalue_2))
    (Variables|Default|SetGallerySaveGame _asbp_photo_gallery)
    ;[1 1 1] Only proceed if random is true or set number is valid
    (if (or (Variables|Default|GetRandomPhoto) (Utilities|Array|IsValidIndex (Variables|/Game/InstantPhotoCamera/Blueprints/BP_PhotoGallery.BP_PhotoGallery_C|GetPictureNumbers (Variables|Default|GetGallerySaveGame)) (Variables|Default|GetPhotoNumber)))
      ;[1 1 1] Import texture by number and set texture
      (if (Utilities|Array|IsValidIndex (Variables|/Game/InstantPhotoCamera/Blueprints/BP_PhotoGallery.BP_PhotoGallery_C|GetPictureNumbers (Variables|Default|GetGallerySaveGame)))
        (bind _returnvalue_3 (Rendering|Material|CreateDynamicMaterialInstance (Variables|Default|GetSM_Photo) 0 0 "None" :!class /Script/Engine.PrimitiveComponent))
        (Variables|Default|SetMaterial _returnvalue_3)
        (bind _returnvalue_4 (Class|KismetRenderingLibrary|ImportFileasTexture2D (Utilities|String|Append (Utilities|String|Append (Class|KismetSystemLibrary|GetProjectSavedDirectory) "/Pictures") "/pic_" (Utilities|String|ToString(Integer) (Utilities|Array|Get(acopy) (Variables|/Game/InstantPhotoCamera/Blueprints/BP_PhotoGallery.BP_PhotoGallery_C|GetPictureNumbers (Variables|Default|GetGallerySaveGame)) (Math|Integer|SelectInt (Math|Random|RandomIntegerinRange 0 (Utilities|Array|LastIndex (Variables|/Game/InstantPhotoCamera/Blueprints/BP_PhotoGallery.BP_PhotoGallery_C|GetPictureNumbers (Variables|Default|GetGallerySaveGame)))) (Variables|Default|GetPhotoNumber) (Variables|Default|GetRandomPhoto)))))))
        (Rendering|Material|SetTextureParameterValue (Variables|Default|GetMaterial) "Picture" _returnvalue_4)
        (Rendering|Material|SetScalarParameterValue (Variables|Default|GetMaterial) "Transition" 1.0 :!class /Script/Engine.MaterialInstanceDynamic)))))

(event EventBeginPlay
  (CallFunction|SetPicture))

(fn ConstructionScript)